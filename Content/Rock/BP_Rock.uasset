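; BP_Rock is a thrown rock projectile that makes noise on impact and can be picked back up by its thrower.
; On spawn it applies its initial velocity to its projectile movement.
; Hits on anything but the instigator while moving fast report AI noise and spawn a Niagara effect scaled to the noise radius.
; Touching the instigator after a short delay restores the character's HasRock flag and destroys the rock.
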(event EventBeginPlay
  (Variables|/Script/Engine.MovementComponent|SetVelocity (Variables|Default|GetProjectileMovement) (Variables|Default|GetInitialVelocity)))

(event Collision|EventHit
  (params (MyComp :type Primitive%20Component%20Object%20Reference) (Other :type Actor%20Object%20Reference) (OtherComp :type Primitive%20Component%20Object%20Reference) (bSelfMoved :type Boolean) (HitLocation :type Vector :default "0, 0, 0") (HitNormal :type Vector :default "0, 0, 0") (NormalImpulse :type Vector :default "0, 0, 0") (Hit :type Hit%20Result%20Structure%20%28by%20ref%29))
  (bind _returnvalue (Transformation|GetActorLocation))
  (bind _returnvalue_2 (Game|GetInstigator))
  (bind _noiseradius (Variables|Default|GetNoiseRadius))
  (if (== Other _returnvalue_2)
    (if (> (Actor|GetGameTimeSinceCreation) 1.0)
      (bind _asbp_third_person_character (Utilities|Casting|CastToBP_ThirdPersonCharacter Other))
      (Variables|/Game/ThirdPerson/Blueprints/BP_ThirdPersonCharacter.BP_ThirdPersonCharacter_C|SetHasRock _asbp_third_person_character true)
      (Actor|DestroyActor))
    (elif (> (Math|Vector|VectorLength (Variables|/Script/Engine.MovementComponent|GetVelocity (Variables|Default|GetProjectileMovement))) 4e+02)
      (Class|Actor|MakeNoise 1.0 _returnvalue_2 _returnvalue _noiseradius "None")
      (bind _returnvalue_3 (Niagara|SpawnSystematLocation "/Game/Rock/NS_NoiseImpact.NS_NoiseImpact" _returnvalue "0, 0, 0" "1.000000,1.000000,1.000000" true false "AutoRelease"))
      (Effects|Components|ParticleSystem|SetFloatParameter _returnvalue_3 "ScaleMax" (* (/ _noiseradius 1e+02) 2.0))
      (Components|Activation|Activate _returnvalue_3 true))))

(fn ConstructionScript)