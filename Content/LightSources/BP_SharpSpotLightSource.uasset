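; Light source Blueprint with a spotlight that can be turned on and off.
; On BeginPlay it sets the spotlight's inner cone to half of ViewAngle, in two identical calls that leave the outer cone untouched.
; It also matches the attenuation radius to the unscaled radius of the EdgeCollisionComponent sphere.
; SetIsTurnedon stores the state in IsTurnedOn and applies it to the spotlight's visibility.
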(event EventBeginPlay
  (bind _viewangle (Variables|Default|GetViewAngle))
  (bind _spotlight (Variables|Default|GetSpotLight))
  (bind _returnvalue (/ _viewangle 2.0))
  (Rendering|Lighting|SetInnerConeAngle _spotlight _returnvalue)
  (Rendering|Lighting|SetInnerConeAngle _spotlight _returnvalue)
  (Rendering|Lighting|SetAttenuationRadius (Variables|Default|GetSpotLight) (Class|SphereComponent|GetUnscaledSphereRadius (Variables|Default|GetEdgeCollisionComponent))))

(event Collision|EventActorBeginOverlap
  (params (OtherActor :type Actor%20Object%20Reference)))

(event EventTick
  (params (DeltaSeconds :type Float%20%28single-precision%29)))

(event EventSetIsTurnedon
  (params (NewState :type Boolean))
  (bind _output_get (Variables|Default|SetIsTurnedOn NewState))
  (Rendering|SetVisibility (Variables|Default|GetSpotLight) _output_get false))

(fn ConstructionScript)